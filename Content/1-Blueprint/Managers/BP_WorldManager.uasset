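; BP_WorldManager starts the app, spawns the UI manager and switches streamed levels between the Perfil view (2D or 3D) and individual "particular" site levels.
; Site levels come from the LermaLevels map, with blocking load/unload behind a loading screen and an IsLoadingParticularLevel guard.
; Switches update the game instance's site ID and UI state, then fire loaded callbacks.
; Alarm manager spawning and compass selection are placeholder prints.
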(event `Start App`
  ;[0.9609 1 0] Inicia world manager
  (`self.Create BP UI Manager`)
  (`self.Load Perfil` false)
  (`self.Spawn Alarmas Manager`)
  (`KismetSystemLibrary.ExecuteConsoleCommand` "r.Steaming.PoolSize 5500" null))

(event `Load Perfil`
  (params (`is 2D?` :type Boolean))
  ;[0 1 0.1524] Carga el nivel del perfil
  (set `self.Is 2D?` `is 2D?`)
  (`self.ShowHideLoadingScreen` true)
  (if (not (`self.is Loading Particular Level`))
    (`GameplayStatics.UnloadStreamLevelBySoftObjectPtr` (`BlueprintMapLibrary.Map_Find` (`self.Lerma Levels`) (`self.Actual Level Id Site`)) true)
    (`GameplayStatics.LoadStreamLevelBySoftObjectPtr` (select `bool` `is 2D?` :`false` (`self.Perfil 3D`) :`true` (`self.Perfil 2D`)) true true)
    (set `self.Actual Level Id Site` (`self.Actual Level Id Site`))
    (set `self.is Perfil Loaded` true)
    (set `self.use Particular` false)
    (`/Game/1-Blueprint/GameInstance/bp_LermaGameInstance.SetCurrentSite Id` (`/Game/1-Blueprint/GeneralFunctions/BP_GeneralFunctions.Get My Game Instance`) 0)
    (`self.Show Brujila 3d o 2d` false)
    (set `self.Actual Level Id Site` (select `bool` `is 2D?` :`false` 101 :`true` 100))
    (`/Game/1-Blueprint/Managers/BP_UI_Manager.OpenUI` (`self.BP UI Manager`))
    (`self.ShowHideLoadingScreen` false)
    (`KismetSystemLibrary.ExecuteConsoleCommand` "r.AntiAliasingMethod 2" null)
    (`self.Set is in Perfil` true)
    (`self.on Perfil Loaded`)))

(event `Load Level By Id Site`
  (params (idSite :type Integer))
  (bind _bp_ui_manager (`self.BP UI Manager`))
  (bind (_value _returnvalue) (`BlueprintMapLibrary.Map_Find` (`self.Lerma Levels`) (`self.Actual Level Id Site`)))
  (bind (_value_2 _returnvalue_2) (`BlueprintMapLibrary.Map_Find` (`self.Lerma Levels`) (`self.Actual Level Id Site`)))
  ;[0 0.4823 1] Carga el nivel de un particular
  (bind _output_get (set `self.idSite` idSite))
  (if (not (== _output_get (`/Game/1-Blueprint/GameInstance/bp_LermaGameInstance.currentSiteId` (`/Game/1-Blueprint/GeneralFunctions/BP_GeneralFunctions.Get My Game Instance`))))
    (`self.Set is in Perfil` false)
    (`self.ShowHideLoadingScreen` true)
    (if (not (`self.is Loading Particular Level`))
      (set `self.is Loading Particular Level` true)
      (set `self.use Particular` true)
      (if (`self.is Perfil Loaded`)
        (`/Game/1-Blueprint/Managers/BP_UI_Manager.Reset Particular` (`self.BP UI Manager`))
        (`GameplayStatics.UnloadStreamLevelBySoftObjectPtr` (`self.Perfil 3D`) true)
        (set `self.is Perfil Loaded` false))
      (if (== (`self.idSite`) (`self.Actual Level Id Site`))
        (set `self.is Loading Particular Level` false)
        (elif _returnvalue_2
          (`GameplayStatics.UnloadStreamLevelBySoftObjectPtr` _value_2 true)
          (if _returnvalue
            (`GameplayStatics.LoadStreamLevelBySoftObjectPtr` _value true true)
            (set `self.Actual Level Id Site` (`self.idSite`))
            (set `self.is Loading Particular Level` false)
            (`/Game/1-Blueprint/Managers/BP_UI_Manager.OpenUI` _bp_ui_manager)
            (`/Game/1-Blueprint/Managers/BP_UI_Manager.Reset Particular` _bp_ui_manager)
            (`/Game/1-Blueprint/Managers/BP_UI_Manager.Show Hide Loading Screen` _bp_ui_manager false)
            (`KismetSystemLibrary.ExecuteConsoleCommand` "r.AntiAliasingMethod 2" null)
            (`/Game/1-Blueprint/GameInstance/bp_LermaGameInstance.SetCurrentSite Id` (`/Game/1-Blueprint/GeneralFunctions/BP_GeneralFunctions.Get My Game Instance`) (`self.Actual Level Id Site`))
            (`self.call on Particular Loaded`)))))))

(event `ShowHideLoadingScreen`
  (params (show :type Boolean))
  ;[0 1 0.08756] Muestra u Oculta la pantalla de carga
  (if (not show)
    (`KismetSystemLibrary.Delay` 0.5))
  (`/Game/1-Blueprint/Managers/BP_UI_Manager.Show Hide Loading Screen` (`/Game/1-Blueprint/GameInstance/bp_LermaGameInstance.Get UI Manager` (`/Game/1-Blueprint/GeneralFunctions/BP_GeneralFunctions.Get My Game Instance`)) show))

(event `Load Level By enum`
  (params (`enum sitio` :type Boolean)))

(fn `Create BP UI Manager`
  (bind _returnvalue (`|SpawnActorFromClass` "/Game/1-Blueprint/Managers/BP_UI_Manager.BP_UI_Manager_C" (`KismetMathLibrary.MakeTransform` (0.0 0.0 0.0)) "Undefined" "MultiplyWithRoot" null null))
  (set `self.BP UI Manager` _returnvalue))

(fn `Set is in Perfil`
  (params (`is In Perfil` :type Boolean))
  (set `/Game/1-Blueprint/Managers/BP_UI_Manager.is in Perfil` `is In Perfil` (`/Game/1-Blueprint/GameInstance/bp_LermaGameInstance.Get UI Manager` (`/Game/1-Blueprint/GeneralFunctions/BP_GeneralFunctions.Get My Game Instance`))))

(fn `Show Brujila 3d o 2d`
  (params (index :type Boolean))
  (`KismetSystemLibrary.PrintString` "Falta elegir brujula"))

(fn `Spawn Alarmas Manager`
  (`KismetSystemLibrary.PrintString` "Falta el actor de Alarmas Manager"))

(fn `UserConstructionScript`)