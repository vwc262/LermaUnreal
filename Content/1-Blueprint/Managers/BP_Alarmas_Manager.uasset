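; Alarm manager that drives the alert sound and screen alert effect for warning and alert levels.
; It binds to game instance data updates and world manager load events, while its update handler always requests the no-warning level, which only stops the sound.
; Warning and alert play a lazily spawned, mute-aware sound and set color, opacity and animation through a post-process Material Parameter Collection.
; Being in the profile view silences the sound and clears the animation.
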(event `self.ReceiveBeginPlay`
  (bind _lermaginstance (`/Game/1-Blueprint/GeneralFunctions/BP_GeneralFunctions.Get My Game Instance`))
  (bind _worldmanager (`/Game/1-Blueprint/GameInstance/bp_LermaGameInstance.GetWorldManager` _lermaginstance))
  ;[1 0 0.001887] Init
  (add `/Game/1-Blueprint/GameInstance/bp_LermaGameInstance.OnUpdateData` _lermaginstance (`|CreateDelegate` :!event `On Update`))
  (add `/Game/1-Blueprint/Managers/BP_WorldManager.on Perfil Loaded` _worldmanager (`|CreateDelegate` :!event `On Update`))
  (add `/Game/1-Blueprint/Managers/BP_WorldManager.call on Particular Loaded` _worldmanager (`|CreateDelegate` :!event `On Update`)))

(event `self.ReceiveDestroyed`
  (bind _lermaginstance (`/Game/1-Blueprint/GeneralFunctions/BP_GeneralFunctions.Get My Game Instance`))
  (bind _worldmanager (`/Game/1-Blueprint/GameInstance/bp_LermaGameInstance.GetWorldManager` _lermaginstance))
  ;[1 0.01876 0] Destroy
  (remove `/Game/1-Blueprint/GameInstance/bp_LermaGameInstance.OnUpdateData` _lermaginstance (`|CreateDelegate` :!event `On Update`))
  (remove `/Game/1-Blueprint/Managers/BP_WorldManager.on Perfil Loaded` _worldmanager (`|CreateDelegate` :!event `On Update`))
  (remove `/Game/1-Blueprint/Managers/BP_WorldManager.call on Particular Loaded` _worldmanager (`|CreateDelegate` :!event `On Update`)))

(event `Stop By Perfil`
  ;[1 0.885 0] Detiene el sonido de la alerta si se entra al perfil
  (`self.SoundAlert`
    (:`then`
      (`AudioComponent.Stop` (`self.SoundAlert`))
      (`self.Set Volume  Sound Alert`)
      (set `self.RepeatAlert` false)
      (`KismetMaterialLibrary.SetScalarParameterValue` "/Game/3-MaterialInstance/PPMaterials/AlertPPMaterialParameters.AlertPPMaterialParameters" "AnimationWeight")
      (`KismetMaterialLibrary.SetScalarParameterValue` "/Game/3-MaterialInstance/PPMaterials/AlertPPMaterialParameters.AlertPPMaterialParameters" "StaticAnimValue"))
    (:`else`)))

(event `On Update`
  ;[1 0.7862 0.07913] Update de la alarma
  (`self.Init Immediatly` "NewEnumerator0"))

(event `Init Immediatly`
  (params (Selection :type "/Game/1-Blueprint/Enums/E_WarningLevels Enum" :default "NewEnumerator0"))
  (bind _is_in_perfil (`/Game/1-Blueprint/Managers/BP_UI_Manager.is in Perfil` (`/Game/1-Blueprint/GameInstance/bp_LermaGameInstance.GetUIManager` (`/Game/1-Blueprint/GeneralFunctions/BP_GeneralFunctions.Get My Game Instance`))))
  ;[1 0.8666 0] Sirve para iniciar el sonido de forma inmediata
  (if (`/Game/1-Blueprint/Managers/BP_UI_Manager.is in Perfil` (`/Game/1-Blueprint/GameInstance/bp_LermaGameInstance.GetUIManager` (`/Game/1-Blueprint/GeneralFunctions/BP_GeneralFunctions.Get My Game Instance`)))
    (`self.Stop By Perfil`)
    (else
      (set `self.Selection` Selection)
      (`/Engine/EditorBlueprintResources/StandardMacros.IsValid` (`self.SoundAlert`)
        (:`Is Valid`
          _)
        (:`Is Not Valid`
          (bind _returnvalue (`GameplayStatics.SpawnSoundAtLocation` "/Game/StarterContent/Audio/Collapse01.Collapse01" (0.0 0.0 0.0) (struct) 1.0 1.0 0.0 null null))
          (bind _output_get (set `self.SoundAlert` _returnvalue))))
      (switch `/Game/1-Blueprint/Enums/E_WarningLevels` (`self.Selection`)
        (:`NewEnumerator0`
          (`AudioComponent.Stop` _output_get))
        (:`NewEnumerator1`
          (`self.Play If Not Playing`)
          (`self.Set Volume  Sound Alert`)
          (`self.Set Alert` _is_in_perfil)
          (set `self.RepeatAlert` true))
        (:`NewEnumerator2`
          (`self.Play If Not Playing`)
          (`self.Set Volume  Sound Alert`)
          (set `self.RepeatAlert` false)
          (`self.Set Alert` _is_in_perfil))))))

(fn `Play If Not Playing`
  (bind _soundalert (`self.SoundAlert`))
  (if (not (`AudioComponent.IsPlaying` _soundalert))
    (`AudioComponent.Play` _soundalert 0.0)))

(fn `Set Alert`
  (params (`is Using Mosaico` :type Boolean))
  (`KismetMaterialLibrary.SetScalarParameterValue` "/Game/3-MaterialInstance/PPMaterials/AlertPPMaterialParameters.AlertPPMaterialParameters" "OpacityScalar" (`KismetMathLibrary.SelectFloat` 0.2 1.0 `is Using Mosaico`))
  (`KismetMaterialLibrary.SetScalarParameterValue` "/Game/3-MaterialInstance/PPMaterials/AlertPPMaterialParameters.AlertPPMaterialParameters" "AnimationWeight" 1.0)
  (`KismetMaterialLibrary.SetScalarParameterValue` "/Game/3-MaterialInstance/PPMaterials/AlertPPMaterialParameters.AlertPPMaterialParameters" "StaticAnimValue" 1.0)
  (`KismetMaterialLibrary.SetVectorParameterValue` "/Game/3-MaterialInstance/PPMaterials/AlertPPMaterialParameters.AlertPPMaterialParameters" "CurrentColor" (select `/Game/1-Blueprint/Enums/E_WarningLevels` (`self.Selection`) :`NewEnumerator1` (`self.Warning`) :`NewEnumerator2` (`self.Alert`))))

(fn `Set Volume  Sound Alert`
  (bind _returnvalue (`KismetMathLibrary.SelectFloat` 0.0 1.0 (`self.Muted`)))
  (`AudioComponent.SetVolumeMultiplier` (`self.SoundAlert`) (select `/Game/1-Blueprint/Enums/E_WarningLevels` (`self.Selection`) :`NewEnumerator1` _returnvalue :`NewEnumerator2` _returnvalue)))

(fn `UserConstructionScript`)