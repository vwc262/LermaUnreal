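; Game instance that loads site infrastructure and live update data from a server and boots the app.
; On init it binds request callbacks and requests infrastructure, whose success starts an update request that refreshes after a delay on success or failure, notifying listeners.
; Site data fills dictionaries keyed by Id, and the first successful update spawns and starts the World Manager once infrastructure has loaded.
; It also lazily spawns the UI Manager and stores the current site Id.
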(event `IniciarServidor`
  ;[0 1 0.2891] Infraestructura
  (`self.FirstServerRequest` (`self.URLInfraestructura`))
  (`self.GetInfraestructura` ""))

(event `self.ReceiveInit`
  ;[1 0.8194 0] Inicio
  (`|ExecutionSequence`
    (:`then_0`
      (`self.AsignarEventos`))
    (:`then_1`
      (`KismetSystemLibrary.Delay` 1.0)
      (`self.IniciarServidor`))))

(event `InfraestructuraFailed`
  ;[1 0 0.04066] Infraestructura Failed
  (set `self.IsErrorEnConexion` true)
  (`KismetSystemLibrary.Delay` 0.2)
  (`self.AsignarSiteDescription`)
  (`self.FirstServerRequest` ""))

(event `InfraestructuraCompleted`
  ;[0 0.5457 1] Infraestructura Completed
  (set `self.IsInfraestructuraCompleted` true)
  (set `self.IsErrorEnConexion` false)
  (`self.GetUpdate` (`self.URLUpdate`)))

(event `AsignarEventos`
  ;[0.08352 1 0] Asignacion de eventos
  (add `self.onInfraestructuraCompleted` (`|CreateDelegate` :!event `InfraestructuraCompleted`))
  (add `self.onInfraestructuraFailed` (`|CreateDelegate` :!event `InfraestructuraFailed`))
  (add `self.onUpdateCompleted` (`|CreateDelegate` :!event `OnUpdate`))
  (add `self.onUpdateFailed` (`|CreateDelegate` :!event `UpdateFailed`)))

(event `UpdateFailed`
  ;[1 0 0.05897] Update Failed
  (set `self.IsErrorEnConexion` true)
  (`KismetSystemLibrary.Delay` 0.5)
  (`self.RefreshFromServer` "")
  ;;[0.843 0 1] Notificacion Error
  (`self.NotificationErrorConnection`))

(event `OnUpdate`
  ;[0.01962 0.456 1] Update Completed
  (`self.IniciarApp`)
  (set `self.IsErrorEnConexion` false)
  (`self.AsignarSiteBase`)
  (`KismetSystemLibrary.Delay` (`KismetMathLibrary.SelectFloat` 2.0 5.0 (`self.PrimeraActualizacion`)))
  ;;[0.7116 0 1] Notificacion Update
  (`self.OnUpdateData`)
  (`self.RefreshFromServer` (`self.URLUpdate`))
  (set `self.PrimeraActualizacion` false))

(event `self.ReceiveShutdown`
  ;[1 0.205 0] Shutdown
  (clear `self.onInfraestructuraCompleted`)
  (clear `self.onInfraestructuraFailed`)
  (clear `self.onUpdateCompleted`)
  (clear `self.onUpdateFailed`))

(fn `AsignarSiteBase`
  (for _array_element (`.Sites` (break `UpdateUnrealSites` (`self.UpdatedData`)))
    (`BlueprintMapLibrary.Map_Add` (`self.SitiosDiccionario`) (`.IdSitio` (break `SiteBase` _array_element)) _array_element)))

(fn `AsignarSiteDescription`
  (for _array_element (`.Sites` (break `Infraestructura` (`self.Infraestructura`)))
    (`BlueprintMapLibrary.Map_Add` (`self.DescripcionSitioDiccionario`) (`.IdSitio` (break `SiteDescription` _array_element)) _array_element)))

(fn `Get UI Manager`
  (returns (NewParam :type "/Game/1-Blueprint/Managers/BP_UI_Manager Object Reference"))
  (`self.bp UI Manager Ref`
    (:`then`
      _)
    (:`else`
      (bind _returnvalue (`|SpawnActorFromClass` "/Game/1-Blueprint/Managers/BP_UI_Manager.BP_UI_Manager_C" (`KismetMathLibrary.MakeTransform` (0.0 0.0 0.0)) "Undefined" "MultiplyWithRoot" null null))
      (set `self.bp UI Manager Ref` _returnvalue)))
  (return (`self.bp UI Manager Ref`)))

(fn `IniciarApp`
  (if (`self.is App iniciada`)
    _
    (elif (`self.isInfraestructuraCompleted`)
      (set `self.is App iniciada` true)
      (`self.AsignarSiteBase`)
      (`self.SpawnWorldManager`))))

(fn `SetCurrentSite Id`
  (params (`id Site` :type Integer))
  (set `self.currentSiteId` `id Site`))

(fn `SpawnWorldManager`
  (bind _returnvalue (`|SpawnActorFromClass` "/Game/1-Blueprint/Managers/BP_WorldManager.BP_WorldManager_C" (`KismetMathLibrary.MakeTransform` (0.0 0.0 0.0)) "Undefined" "MultiplyWithRoot" null null))
  (`/Game/1-Blueprint/Managers/BP_WorldManager.Start App` _returnvalue))