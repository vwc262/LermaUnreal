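; BP_GeneralFunctions is a collection of shared helper functions for game instance access, text formatting and site status.
; GetMyGameInstance returns the game instance cast to bp_LermaGameInstance.
; IsSiteOnline uses it to look up a site by ID and returns its Enlace field when found.
; MilesSinComas strips commas from a value's text, while GetAlarmBySite is an empty stub.
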(fn `Get My Game Instance`
  (returns (LermaGInstance :type "/Game/1-Blueprint/GameInstance/bp_LermaGameInstance Object Reference"))
  (bind (_asbp_lerma_game_instance _bsuccess) (cast `/Game/1-Blueprint/GameInstance/bp_LermaGameInstance` (`GameplayStatics.GetGameInstance` null) :!pure true))
  (if _bsuccess
    (return _asbp_lerma_game_instance)))

(fn `GetAlarmBySite`
  (params (`ID Sitio` :type Integer))
  (locals (_CountCritical :type Integer) (_CountWarning :type Integer)))

(fn `IsSiteOnline`
  (params (`ID Sitio` :type Integer))
  (returns (IsOnline :type Boolean))
  (bind (_sitio _found) (`/Game/1-Blueprint/GameInstance/bp_LermaGameInstance.GetSite` (`self.Get My Game Instance` null) `ID Sitio`))
  (if _found
    (return (`.Enlace` (break `SiteBase` _sitio)))))

(fn `MilesSinComas`
  (params (Value :type Text))
  (returns (NewValue :type Text))
  (return (`KismetTextLibrary.Conv_StringToText` (`KismetStringLibrary.Replace` (`KismetTextLibrary.Conv_TextToString` Value) ","))))